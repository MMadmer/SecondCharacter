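; Game mode that runs the game's task flow, starting with a storage task on BeginPlay.
; MakeTask constructs a task object from a class, binds its finished event, stores it as current, starts it and broadcasts OnTaskCreated.
; FinishTask clears the current task and broadcasts OnTaskFinished with it, first asking the level's BP_Spawner to spawn a client unless it was a main hero task.
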(event `self.ReceiveBeginPlay`
  (`self.MakeTask` "/Game/SecondCharacter/Blueprints/Tasks/BP_StorageGameTask.BP_StorageGameTask_C"))

(fn `FinishTask`
  (locals (LastTask :type "SCBaseTask Object Reference"))
  (bind _output_get (set `local.LastTask` (`self.CurrentTask`)))
  (`|ExecutionSequence`
    (:`then_0`
      (cast `/Game/SecondCharacter/Blueprints/Tasks/BP_MainHeroTask` (`self.CurrentTask`)
        (:`CastFailed`
          (`self.SpawnClient`))))
    (:`then_1`
      (set `self.CurrentTask` null)
      (`self.OnTaskFinished` _output_get))))

(fn `GetCurrentTask`
  (returns (CurrentTask :type "SCBaseTask Object Reference"))
  (return (`self.CurrentTask`)))

(fn `MakeTask`
  (params (Task :type "SCBaseTask Class Reference"))
  (if (`KismetSystemLibrary.IsValidClass` Task)
    (bind _returnvalue (`|GenericCreateObject` self Task))
    (add `SCBaseTask.OnTaskFinished` _returnvalue (`|CreateDelegate` :!event `FinishTask`))
    (bind _output_get (set `self.CurrentTask` _returnvalue))
    (`SCBaseTask.StartTask` _output_get)
    (`self.OnTaskCreated` _output_get)))

(fn `SpawnClient`
  (bind _returnvalue (`GameplayStatics.GetActorOfClass` "/Game/SecondCharacter/Blueprints/NPC/BP_Spawner.BP_Spawner_C"))
  (`/Engine/EditorBlueprintResources/StandardMacros.IsValid` _returnvalue
    (:`Is Valid`
      (`/Game/SecondCharacter/Blueprints/NPC/BP_Spawner.Spawn` _returnvalue))))

(fn `UserConstructionScript`)