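; BPC_StorageComponent is a component that stores a single normalized amount and can pass it between storage components.
; SetValue clamps the amount to 0–1, records the previous value and fires OnValueChanged only when the value changes.
; Transfer pulls from a valid source component through its GrabValue, which deducts and returns the grabbed amount, then adds that amount to its own value.
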(fn `GetValue`
  (returns (Value :type "Float (double-precision)"))
  (return (`self.Value`)))

(fn `GrabValue`
  (params (Value :type "Float (double-precision)"))
  (returns (GrabbedValue :type "Float (double-precision)"))
  (locals (Grabbed :type "Float (double-precision)"))
  (bind _value (`self.Value`))
  (bind _output_get (set `local.Grabbed` (select `bool` (>= (- _value Value) 0.0) :`false` (- Value _value) :`true` Value)))
  (`self.SetValue` (- (`self.Value`) _output_get))
  (return _output_get))

(fn `SetValue`
  (params (NewValue :type "Float (double-precision)"))
  (locals (LastValue :type "Float (double-precision)"))
  (bind _output_get (set `local.LastValue` (`self.Value`)))
  (bind _output_get_2 (set `self.Value` (`KismetMathLibrary.FClamp` NewValue)))
  (if (!= _output_get_2 _output_get)
    (`self.OnValueChanged` _output_get_2)))

(fn `Transfer`
  (params (FromComp :type "/Game/SecondCharacter/Blueprints/Components/BPC_StorageComponent Object Reference") (Value :type "Float (double-precision)"))
  (`/Engine/EditorBlueprintResources/StandardMacros.IsValid` FromComp
    (:`Is Valid`
      (bind _grabbedvalue (`self.GrabValue` FromComp Value))
      (`self.SetValue` (+ (`self.Value`) _grabbedvalue)))))