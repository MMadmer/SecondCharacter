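; A level trigger that sells items entering its box during a sell task, paying the player and removing the item.
; On overlap, it accepts only BPI_Sells actors that are on the item list of the game mode's current BP_SellTask and report they can be sold.
; It adds the item's cost to player 0's BP_PlayerState, notifies the task of the sale, then destroys the actor.
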(event `self.Box.OnComponentBeginOverlap`
  (params (OverlappedComponent :type "PrimitiveComponent Object Reference") (OtherActor :type "Actor Object Reference") (OtherComp :type "PrimitiveComponent Object Reference") (OtherBodyIndex :type Integer) (bFromSweep :type Boolean) (SweepResult :type "HitResult Structure (by ref)"))
  (if (`KismetSystemLibrary.DoesImplementInterface` OtherActor "/Game/SecondCharacter/Blueprints/Interfaces/BPI_Sells.BPI_Sells_C")
    (bind _asbp_game_mode_base (cast `/Game/SecondCharacter/Blueprints/BP_GameModeBase` (`GameplayStatics.GetGameMode`)))
    (bind _asbp_sell_task (cast `/Game/SecondCharacter/Blueprints/Tasks/BP_SellTask` (`/Game/SecondCharacter/Blueprints/BP_GameModeBase.GetCurrentTask` _asbp_game_mode_base)))
    (bind _items (`/Game/SecondCharacter/Blueprints/Tasks/BP_SellTask.GetItemsToSell` _asbp_sell_task))
    (if (`KismetArrayLibrary.Array_Contains` _items OtherActor)
      (bind _can (message `/Game/SecondCharacter/Blueprints/Interfaces/BPI_Sells.CanBeSold` OtherActor))
      (if _can
        (bind _cost (message `/Game/SecondCharacter/Blueprints/Interfaces/BPI_Sells.GetCost` OtherActor))
        (bind _asbp_player_state (cast `/Game/SecondCharacter/Blueprints/Player/BP_PlayerState` (`GameplayStatics.GetPlayerState` 0)))
        (`/Game/SecondCharacter/Blueprints/Player/BP_PlayerState.AddMoney` _asbp_player_state _cost)
        (`/Game/SecondCharacter/Blueprints/Tasks/BP_SellTask.ItemSold` _asbp_sell_task OtherActor)
        (`self.K2_DestroyActor` OtherActor)))))

(fn `UserConstructionScript`)