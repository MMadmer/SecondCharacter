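; BP_ColorStation is a colored refill station that docks a flask and steadily fills its storage component.
; On box overlap it accepts an actor with a matching FlaskTag, or retags an empty BP_Flask, then attaches it to the mesh via a physics constraint.
; Tick raises the linked storage value at Speed until the constraint breaks, which unlinks it and starts a short reconnect cooldown.
; The construction script applies ColorMat to the mesh.
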(event `self.ReceiveTick`
  (params (DeltaSeconds :type "Float (single-precision)"))
  (bind _linkedstorage (`self.LinkedStorage`)
    (:`then`
      (`/Game/SecondCharacter/Blueprints/Components/BPC_StorageComponent.SetValue` _linkedstorage (+ (`/Game/SecondCharacter/Blueprints/Components/BPC_StorageComponent.GetValue` _linkedstorage) (* DeltaSeconds (`self.Speed`)))))
    (:`else`)))

(event `self.Box.OnComponentBeginOverlap`
  (params (OverlappedComponent :type "PrimitiveComponent Object Reference") (OtherActor :type "Actor Object Reference") (OtherComp :type "PrimitiveComponent Object Reference") (OtherBodyIndex :type Integer) (bFromSweep :type Boolean) (SweepResult :type "HitResult Structure (by ref)"))
  (bind _returnvalue (`self.GetComponentByClass` OtherActor "/Game/SecondCharacter/Blueprints/Components/BPC_StorageComponent.BPC_StorageComponent_C"))
  (if (`self.CanConnect`)
    (if (`self.ActorHasTag` OtherActor (`self.FlaskTag`))
      (bind _asprimitive_component (cast `PrimitiveComponent` (`Actor.RootComponent` OtherActor) :!label _label))
      (`PhysicsConstraintComponent.SetConstrainedComponents` (`self.PhysicsConstraint`) _asprimitive_component "None" (`self.StaticMesh`) "None")
      (set `self.CanConnect` false)
      (set `self.LinkedStorage` _returnvalue)
      (else
        (`/Engine/EditorBlueprintResources/StandardMacros.IsValid` _returnvalue
          (:`Is Valid`
            (if (`KismetMathLibrary.NearlyEqual_FloatFloat` (`/Game/SecondCharacter/Blueprints/Components/BPC_StorageComponent.GetValue` _returnvalue))
              (bind _asbp_flask (cast `/Game/SecondCharacter/Blueprints/LevelObjects/Liquid/BP_Flask` OtherActor))
              (`/Game/SecondCharacter/Blueprints/LevelObjects/Liquid/BP_Flask.SetFlaskTag` _asbp_flask (`self.FlaskTag`))
              (goto _label))))))))

(event `self.PhysicsConstraint.OnConstraintBroken`
  (params (ConstraintIndex :type Integer))
  (set `self.CanConnect` false)
  (`KismetSystemLibrary.K2_SetTimerDelegate` (delegate `Restore`) 5.0)
  (set `self.LinkedStorage` null))

(event `Restore`
  (set `self.CanConnect` true))

(fn `UserConstructionScript`
  (`PrimitiveComponent.SetMaterial` (`self.StaticMesh`) 0 (`self.ColorMat`)))