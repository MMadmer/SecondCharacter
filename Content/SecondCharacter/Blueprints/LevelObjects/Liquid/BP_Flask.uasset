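; BP_Flask is a grabbable liquid flask that can be sold during a color-selling task.
; Its storage component drives the material's Fill parameter and, on emptying, resets the flask tag and actor tags to just "grab".
; Setting the flask tag adds it as an actor tag and selects a red, green or blue liquid material.
; It is sellable only when full and its color is among those the game mode's current task requests.
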(event `self.BPC_StorageComponent.OnValueChanged`
  (params (NewValue :type "Float (double-precision)"))
  (bind _tags (`self.Tags`))
  (bind _staticmesh (`self.StaticMesh`))
  (bind _returnvalue (`PrimitiveComponent.GetMaterial` _staticmesh 0))
  (`|ExecutionSequence`
    (:`then_0`
      (`/Engine/EditorBlueprintResources/StandardMacros.IsValid` _returnvalue
        (:`Is Valid`
          (bind _returnvalue_2 (`PrimitiveComponent.CreateDynamicMaterialInstance` _staticmesh 0 _returnvalue "None"))
          (`/Engine/EditorBlueprintResources/StandardMacros.IsValid` _returnvalue_2
            (:`Is Valid`
              (`MaterialInstanceDynamic.SetScalarParameterValue` _returnvalue_2 "Fill" NewValue))))))
    (:`then_1`
      (if (`KismetMathLibrary.NearlyEqual_FloatFloat` NewValue)
        (set `self.FlaskTag` "None")
        (`KismetArrayLibrary.Array_Clear` _tags)
        (`KismetArrayLibrary.Array_AddUnique` _tags "grab")))))

(fn `CanBeSold`
  (returns (Can :type Boolean))
  (bind _asbp_game_mode_base (cast `/Game/SecondCharacter/Blueprints/BP_GameModeBase` (`GameplayStatics.GetGameMode`))
    (:`then`
      (bind _asbp_colors_sell_task (cast `/Game/SecondCharacter/Blueprints/Tasks/BP_ColorsSellTask` (`/Game/SecondCharacter/Blueprints/BP_GameModeBase.GetCurrentTask` _asbp_game_mode_base))
        (:`then`
          (bind _colors (`/Game/SecondCharacter/Blueprints/Tasks/BP_ColorsSellTask.GetColorsToSell` _asbp_colors_sell_task))
          (return (and (`KismetArrayLibrary.Array_Contains` _colors (`self.FlaskTag`)) (>= (`/Game/SecondCharacter/Blueprints/Components/BPC_StorageComponent.GetValue` (`self.BPC_StorageComponent`)) 1.0))))
        (:`CastFailed`
          _)))
    (:`CastFailed`
      _))
  (return false))

(fn `GetCost`
  (returns (Cost :type Integer))
  (return 100))

(fn `GetFlaskTag`
  (returns (FlaskTag :type Name))
  (return (`self.FlaskTag`)))

(fn `GetItemName`
  (returns (Name :type Text))
  (return ""))

(fn `SetFlaskTag`
  (params (FlaskTag :type Name))
  (`self.SetLiquidMat` (`KismetStringLibrary.Conv_NameToString` FlaskTag))
  (`KismetArrayLibrary.Array_AddUnique` (`self.Tags`) FlaskTag)
  (set `self.FlaskTag` FlaskTag))

(fn `SetLiquidMat`
  (params (Channel :type String))
  (bind _staticmesh (`self.StaticMesh`))
  (switch `string` Channel
    (:`red`
      (`PrimitiveComponent.SetMaterial` _staticmesh 0 "/Game/Assets/Materials/MI_Red.MI_Red"))
    (:`green`
      (`PrimitiveComponent.SetMaterial` _staticmesh 0 "/Game/Assets/Materials/MI_Green.MI_Green"))
    (:`blue`
      (`PrimitiveComponent.SetMaterial` _staticmesh 0 "/Game/Assets/Materials/MI_Blue.MI_Blue"))))

(fn `UserConstructionScript`
  (`PrimitiveComponent.SetMaterial` (`self.StaticMesh`) 0 (`self.ColorMat`)))