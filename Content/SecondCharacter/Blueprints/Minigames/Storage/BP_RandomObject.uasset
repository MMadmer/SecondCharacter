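; BP_RandomObject is a physics prop for the storage minigame that takes on a random mesh from its Meshes list when play begins.
; The construction script blocking-loads the first mesh as a preview.
; BeginPlay async-loads a random entry, applies it, gives the actor a random rotation and enables physics simulation.
; The actor destroys itself if the list is empty or no valid mesh results.
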(event `self.ReceiveBeginPlay`
  (bind _meshes (`self.Meshes`))
  (bind _staticmesh (`self.StaticMesh`))
  (if (`KismetArrayLibrary.Array_IsNotEmpty` _meshes)
    (bind _object (`|LoadAsset` (`KismetArrayLibrary.Array_Random` _meshes))
      (:`Completed`
        (bind _asstatic_mesh (cast `StaticMesh` _object)
          (:`then`
            (`StaticMeshComponent.SetStaticMesh` _staticmesh _asstatic_mesh)
            (`StaticMeshComponent.StaticMesh` _staticmesh
              (:`then`
                (`self.K2_SetActorRotation` (`KismetMathLibrary.RandomRotator` true) true)
                (`PrimitiveComponent.SetSimulatePhysics` _staticmesh true))
              (:`else`
                (`self.K2_DestroyActor`))))
          (:`CastFailed`
            (`self.K2_DestroyActor`)))))
    (else
      (`self.K2_DestroyActor`))))

(fn `UserConstructionScript`
  (bind _meshes (`self.Meshes`))
  (if (`KismetArrayLibrary.Array_IsNotEmpty` _meshes)
    (bind _returnvalue (`KismetSystemLibrary.LoadAsset_Blocking` (`|GetArrayItem` _meshes)))
    (bind _asstatic_mesh (cast `StaticMesh` _returnvalue))
    (`StaticMeshComponent.SetStaticMesh` (`self.StaticMesh`) _asstatic_mesh)))