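; BP_Storage is a storage zone for a minigame that signals when items with a matching tag enter or leave it.
; Its Box component's overlap events filter actors by CheckTag and fire the OnItemEntered and OnItemLeft dispatchers.
; On BeginPlay it collapses the box to zero and restores its extent with an overlap update, apparently to register items already inside at start.
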(event `self.ReceiveBeginPlay`
  (bind _box (`self.Box`))
  (bind _output_get (set `self.OriginalExtent` (`BoxComponent.BoxExtent` _box)))
  (`BoxComponent.SetBoxExtent` _box (0.0 0.0 0.0) false)
  (`BoxComponent.SetBoxExtent` _box _output_get true))

(event `self.Box.OnComponentBeginOverlap`
  (params (OverlappedComponent :type "PrimitiveComponent Object Reference") (OtherActor :type "Actor Object Reference") (OtherComp :type "PrimitiveComponent Object Reference") (OtherBodyIndex :type Integer) (bFromSweep :type Boolean) (SweepResult :type "HitResult Structure (by ref)"))
  (if (`self.ActorHasTag` OtherActor (`self.CheckTag`))
    (`self.OnItemEntered`)))

(event `self.Box.OnComponentEndOverlap`
  (params (OverlappedComponent :type "PrimitiveComponent Object Reference") (OtherActor :type "Actor Object Reference") (OtherComp :type "PrimitiveComponent Object Reference") (OtherBodyIndex :type Integer))
  (if (`self.ActorHasTag` OtherActor (`self.CheckTag`))
    (`self.OnItemLeft`)))

(fn `UserConstructionScript`)