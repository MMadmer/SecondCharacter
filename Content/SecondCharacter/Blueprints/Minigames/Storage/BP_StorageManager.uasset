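; BP_StorageManager tracks items across all storage spots in a storage minigame and signals when enough have been collected.
; On BeginPlay it finds every BP_Storage in the level and binds to their item-entered and item-left events.
; Those events raise or lower a shared count, and the first time it reaches MaxItems the manager fires its OnItemsCollected dispatcher, guarded by a DoOnce.
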(event `self.ReceiveBeginPlay`
  (bind _outactors (`GameplayStatics.GetAllActorsOfClass` "/Game/SecondCharacter/Blueprints/Minigames/Storage/BP_Storage.BP_Storage_C"))
  (for _array_element _outactors
    (add `/Game/SecondCharacter/Blueprints/Minigames/Storage/BP_Storage.OnItemEntered` _array_element (delegate `OnItemEntered`))
    (add `/Game/SecondCharacter/Blueprints/Minigames/Storage/BP_Storage.OnItemLeft` _array_element (delegate `OnItemLeft`))))

(event `OnItemEntered`
  (bind _result (`/Engine/EditorBlueprintResources/StandardMacros.IncrementInt` (`self.CurrentItems`))
    (:`  `
      (if (>= _result (`self.MaxItems`))
        (`/Engine/EditorBlueprintResources/StandardMacros.DoOnce` false
          (:`Completed`
            (`self.OnItemsCollected`)))))))

(event `OnItemLeft`
  (`/Engine/EditorBlueprintResources/StandardMacros.DecrementInt` (`self.CurrentItems`)))

(fn `UserConstructionScript`)