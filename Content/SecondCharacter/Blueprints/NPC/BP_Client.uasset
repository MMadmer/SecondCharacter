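; BP_Client is a client NPC that takes on a selling task when product storage exists in the level.
; Its CallTask override looks up a BP_StorageProduct actor and, if one is valid, randomly sets Task to either BP_ColorsSellTask or BP_SellTask.
; It then always runs the parent CallTask, leaving all other behavior to the parent class.
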(event `self.ReceiveBeginPlay`
  (`parent.ReceiveBeginPlay`))

(fn `CallTask`
  (`|ExecutionSequence`
    (:`then_0`
      (bind _returnvalue (`GameplayStatics.GetActorOfClass` "/Game/SecondCharacter/Blueprints/LevelObjects/Products/BP_StorageProduct.BP_StorageProduct_C"))
      (`/Engine/EditorBlueprintResources/StandardMacros.IsValid` _returnvalue
        (:`Is Valid`
          (set `self.Task` (select `bool` (`KismetMathLibrary.RandomBool`) :`false` "/Game/SecondCharacter/Blueprints/Tasks/BP_SellTask.BP_SellTask_C" :`true` "/Game/SecondCharacter/Blueprints/Tasks/BP_ColorsSellTask.BP_ColorsSellTask_C" :!type "SCBaseTask Class Reference")))))
    (:`then_1`
      (`parent.CallTask`))))

(fn `UserConstructionScript`
  (`parent.UserConstructionScript`))