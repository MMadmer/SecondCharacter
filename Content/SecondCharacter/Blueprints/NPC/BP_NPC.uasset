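; NPC actor that rocks its static mesh while moving and can hand its Task to the game mode.
; Tick compares the location with the last frame's and, on movement, starts a DoOnce-gated timeline that rolls the mesh up to MaxAngle and reverses back.
; When the reverse finishes, MaxAngle is modified and the gate resets for the next swing.
; CallTask passes Task to BP_GameModeBase's MakeTask.
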(event `self.ReceiveBeginPlay`
  (set `self.LastLocation` (`self.K2_GetActorLocation`)))

(event `self.ReceiveTick`
  (params (DeltaSeconds :type "Float (single-precision)"))
  (`|ExecutionSequence`
    (:`then_0`
      (if (not (`KismetMathLibrary.Vector_IsNearlyZero` (- (`self.K2_GetActorLocation`) (`self.LastLocation`))))
        (`/Engine/EditorBlueprintResources/StandardMacros.DoOnce` false :!label _label
          (:`Completed`
            (bind (_direction _alpha) (`Timeline|Anim` :!label _label_2)
              (:`Update`
                (`SceneComponent.K2_SetRelativeRotation` (`self.StaticMesh`) (`KismetMathLibrary.MakeRotator` (* _alpha (`self.MaxAngle`))) false false))
              (:`Finished`
                (switch `ETimelineDirection` _direction
                  (:`Forward`
                    (goto _label_2 :!via `Reverse`))
                  (:`Backward`
                    (`/Engine/EditorBlueprintResources/StandardMacros.NegateFloat` (`self.MaxAngle`)
                      (:`  `
                        (goto _label :!via `Reset`)))))))))))
    (:`then_1`
      (set `self.LastLocation` (`self.K2_GetActorLocation`)))))

(fn `CallTask`
  (bind _asbp_game_mode_base (cast `/Game/SecondCharacter/Blueprints/BP_GameModeBase` (`GameplayStatics.GetGameMode`)))
  (`/Game/SecondCharacter/Blueprints/BP_GameModeBase.MakeTask` _asbp_game_mode_base (`self.Task`)))

(fn `UserConstructionScript`)