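; NPC spawner that creates one character at a time and moves it along a spline.
; Spawn destroys the current NPC, spawns the ToSpawn class at the spline component's transform, then resets the travel distance and completion latch.
; Tick advances the distance by Speed, setting the NPC's location and rotation from the spline, raised by its capsule half-height.
; At the spline's end, a DoOnce triggers the NPC's CallTask.
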(event `self.ReceiveBeginPlay`)

(event `self.ReceiveTick`
  (params (DeltaSeconds :type "Float (single-precision)"))
  (bind _spline (`self.Spline`))
  (bind _currentnpc (`self.CurrentNPC`)
    (:`then`
      (bind _output_get (set `self.Distance` (+ (`self.Distance`) (* DeltaSeconds (`self.Speed`)))))
      (bind (_returnvalue_location _returnvalue_rotation) (`KismetMathLibrary.BreakTransform` (`SplineComponent.GetTransformAtDistanceAlongSpline` _spline _output_get "World" false)))
      (`self.K2_SetActorLocationAndRotation` _currentnpc (+ _returnvalue_location (`KismetMathLibrary.MakeVector` 0.0 0.0 (`CapsuleComponent.GetScaledCapsuleHalfHeight` (`/Game/SecondCharacter/Blueprints/NPC/BP_NPC.Capsule` _currentnpc)))) _returnvalue_rotation false false)
      (if (>= (`SplineComponent.GetTimeAtDistanceAlongSpline` _spline _output_get) 1.0)
        (`/Engine/EditorBlueprintResources/StandardMacros.DoOnce` false :!label _label
          (:`Completed`
            (`/Game/SecondCharacter/Blueprints/NPC/BP_NPC.CallTask` (`self.CurrentNPC`))))))
    (:`else`)))

(event `Spawn`
  (bind _tospawn (`self.ToSpawn`))
  (bind _spline (`self.Spline`))
  (bind _currentnpc (`self.CurrentNPC`)
    (:`then`
      (`self.K2_DestroyActor` _currentnpc))
    (:`else`
      _))
  (if (`KismetSystemLibrary.IsValidClass` _tospawn)
    (bind _returnvalue (`|SpawnActorFromClass` _tospawn (`KismetMathLibrary.MakeTransform` (`SceneComponent.K2_GetComponentLocation` _spline) (`SceneComponent.K2_GetComponentRotation` _spline)) "AlwaysSpawn" "MultiplyWithRoot" null null))
    (bind _output_get (set `self.CurrentNPC` _returnvalue))
    (`/Engine/EditorBlueprintResources/StandardMacros.IsValid` _output_get
      (:`Is Valid`
        (`self.K2_SetActorLocation` _output_get (+ (`self.K2_GetActorLocation` _output_get) (`KismetMathLibrary.MakeVector` 0.0 0.0 (`CapsuleComponent.GetScaledCapsuleHalfHeight` (`/Game/SecondCharacter/Blueprints/NPC/BP_NPC.Capsule` _output_get)))) false false)
        (set `self.Distance` 0.0)
        (goto _label :!via `Reset`)))))

(fn `UserConstructionScript`)