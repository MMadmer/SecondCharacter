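; BP_PlayerState is a player state Blueprint that holds the player's money.
; AddMoney applies a value to Money, clamps the result at zero, and calls the OnMoneyChanged dispatcher only when the balance actually changes, passing a constant zero rather than the new amount.
; GetMoney returns the current balance, and the event graph has no active logic.
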(fn `AddMoney`
  (params (Value :type Integer))
  (locals (LastMoney :type Integer))
  (bind _output_get (set `local.LastMoney` (`self.Money`)))
  (bind _output_get_2 (set `self.Money` (`KismetMathLibrary.Max` (+ Value (`self.Money`)))))
  (if (!= _output_get_2 _output_get)
    (`self.OnMoneyChanged` 0)))

(fn `GetMoney`
  (returns (Money :type Integer))
  (return (`self.Money`)))

(fn `UserConstructionScript`)