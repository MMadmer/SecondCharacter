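; Task for the second character that asks for a random set of colors to be sold.
; On start it draws one to three entries from AvailableColors into ColorsToSell, with duplicates possible.
; GetDescription joins the remaining colors into a comma-separated Russian "Sell" prompt.
; ColorSold removes one matching entry per sale and signals task completion when the list empties.
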(event `self.StartTask`
  (for _index (range (+ (`KismetMathLibrary.RandomIntegerInRange` 1 2) 1))
    (if (> _index 0)
      (`KismetArrayLibrary.Array_Add` (`self.ColorsToSell`) (`KismetArrayLibrary.Array_Random` (`self.AvailableColors`)) :!label _label)
      (elif (`KismetMathLibrary.RandomBool`)
        (goto _label)))))

(fn `ColorSold`
  (params (Color :type Name))
  (bind _colorstosell (`self.ColorsToSell`))
  (bind _returnvalue (`KismetArrayLibrary.Array_Find` _colorstosell Color))
  (if (>= _returnvalue 0)
    (`KismetArrayLibrary.Array_Remove` _colorstosell _returnvalue)
    (if (`KismetArrayLibrary.Array_IsEmpty` _colorstosell)
      (`self.OnTaskFinished`))))

(fn `GetColorsToSell`
  (returns (Colors :type "Array of Name"))
  (return (`self.ColorsToSell`)))

(fn `GetDescription`
  (returns (ReturnValue :type Text))
  (locals (Result :type Text))
  (for (_array_element _array_index) (`self.ColorsToSell`)
    (bind _returnvalue (`KismetTextLibrary.Conv_NameToText` _array_element))
    (set `local.Result` (`|FormatText` "{Result}{New}" (`local.Result`) (select `bool` (> _array_index 0) :`false` _returnvalue :`true` (`|FormatText` ", {Name}" _returnvalue)))))
  (return (`|FormatText` "Продайте {item}" (`local.Result`))))