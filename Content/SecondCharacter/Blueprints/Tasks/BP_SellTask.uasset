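; Sell task that asks the player to sell products chosen from the BP_StorageProduct actors in the level.
; On start it always takes the first actor found, then adds later ones on a coin flip until MaxItems is reached.
; It builds a Russian "Sell …" description from the comma-joined item names.
; ItemSold removes each sold item and fires OnTaskFinished once the list is empty.
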(event `self.StartTask`
  (bind _returnvalue (`self.GetAllActorsOfClass` "/Game/SecondCharacter/Blueprints/LevelObjects/Products/BP_StorageProduct.BP_StorageProduct_C"))
  (for (_array_element _array_index) _returnvalue
    (if (< (`self.CurrentItems`) (`self.MaxItems`))
      (if (> _array_index 0)
        (if (`KismetMathLibrary.RandomBool`)
          (`KismetArrayLibrary.Array_Add` (`self.ItemsToSell`) _array_element :!label _label)
          (`/Engine/EditorBlueprintResources/StandardMacros.IncrementInt` (`self.CurrentItems`)))
        (else
          (goto _label)))
      (else
        (break)))))

(fn `GetDescription`
  (returns (ReturnValue :type Text))
  (locals (Result :type Text))
  (for (_array_element _array_index) (`self.ItemsToSell`)
    (bind _name (message `/Game/SecondCharacter/Blueprints/Interfaces/BPI_Sells.GetItemName` _array_element))
    (set `local.Result` (`|FormatText` "{Result}{New}" (`local.Result`) (select `bool` (> _array_index 0) :`false` _name :`true` (`|FormatText` ", {Name}" _name)))))
  (return (`|FormatText` "Продайте {item}" (`local.Result`))))

(fn `GetItemsToSell`
  (returns (Items :type "Array of Actor Object Reference"))
  (return (`self.ItemsToSell`)))

(fn `ItemSold`
  (params (Item :type "Actor Object Reference"))
  (bind _itemstosell (`self.ItemsToSell`))
  (`KismetArrayLibrary.Array_RemoveItem` _itemstosell Item)
  (if (`KismetArrayLibrary.Array_IsEmpty` _itemstosell)
    (`self.OnTaskFinished`)))