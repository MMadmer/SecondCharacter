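; BP_StorageGameTask is a game task that tracks items being put away into storage and finishes once all are stored.
; On StartTask it counts actors tagged "storage" as the target and binds to every BP_Storage's item-entered and item-left events.
; Those events adjust the current count, and reaching the target fires the task-finished dispatcher once.
; GetDescription reports progress as Russian text showing current and maximum items.
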(event `self.StartTask`
  (bind _returnvalue (`self.GetAllActorsWithTag` "storage"))
  (set `self.MaxItems` (`KismetArrayLibrary.Array_Length` _returnvalue))
  (bind _returnvalue_2 (`self.GetAllActorsOfClass` "/Game/SecondCharacter/Blueprints/Minigames/Storage/BP_Storage.BP_Storage_C"))
  (for _array_element _returnvalue_2
    (add `/Game/SecondCharacter/Blueprints/Minigames/Storage/BP_Storage.OnItemEntered` _array_element (delegate `OnItemEntered`))
    (add `/Game/SecondCharacter/Blueprints/Minigames/Storage/BP_Storage.OnItemLeft` _array_element (delegate `OnItemLeft`))))

(event `OnItemEntered`
  (bind _result (`/Engine/EditorBlueprintResources/StandardMacros.IncrementInt` (`self.CurrentItems`))
    (:`  `
      (if (>= _result (`self.MaxItems`))
        (`/Engine/EditorBlueprintResources/StandardMacros.DoOnce` false
          (:`Completed`
            (`self.OnTaskFinished`)))))))

(event `OnItemLeft`
  (`/Engine/EditorBlueprintResources/StandardMacros.DecrementInt` (`self.CurrentItems`)))

(fn `GetDescription`
  (returns (ReturnValue :type Text))
  (return (`|FormatText` "Убрано товаров: {Current} из {Max}" (`self.CurrentItems`) (`self.MaxItems`))))